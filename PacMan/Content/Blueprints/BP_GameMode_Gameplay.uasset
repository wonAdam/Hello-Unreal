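; Gameplay game mode that opens the level with a timed camera transition before handing control to the player.
; On BeginPlay it disables player input, spawns a camera actor at the gameplay camera transform and slowly blends the view to it.
; After a delay slightly longer than the blend, it re-enables input and sets the movement flag on BP_Player.
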(event `self.ReceiveBeginPlay`
  (bind _returnvalue (`GameplayStatics.GetPlayerCharacter` 0))
  (`|ExecutionSequence`
    (:`then_1`
      ;[1 1 0] Gameplay Camera
      (`self.DisableInput` (`GameplayStatics.GetPlayerCharacter` 0) (`GameplayStatics.GetPlayerController` 0))
      (bind _returnvalue_2 (`|SpawnActorFromClass` "/Script/Engine.CameraActor" (`KismetMathLibrary.MakeTransform` (`self.CamGameplay_Loc`) (`self.CamGameplay_Rot`)) "Undefined" "OverrideRootScale" null null))
      (`PlayerController.SetViewTargetWithBlend` (`GameplayStatics.GetPlayerController` 0) _returnvalue_2 6.8 "VTBlend_Linear" 0.0 false)
      (`KismetSystemLibrary.Delay` 7.0)
      (`self.EnableInput` _returnvalue (`GameplayStatics.GetPlayerController` 0))
      (bind _asbp_player (cast `/Game/Blueprints/BP_Player` _returnvalue))
      (set `/Game/Blueprints/BP_Player.bAllowToMove?` true _asbp_player))))

(fn `UserConstructionScript`)