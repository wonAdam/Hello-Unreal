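; Rifle weapon Blueprint that fires a cosmetic hitscan shot through its PullTrigger event.
; Each shot plays a muzzle effect at the mesh socket, then, if the owner is a Pawn, line-traces up to MaxRange from player 0's camera along that player's view direction.
; A hit spawns the MuzzleSplash effect at the impact point; no damage is applied, and the debug draw nodes are disconnected.
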(event `self.BP_PullTrigger`
  (bind _returnvalue (`PlayerCameraManager.GetCameraLocation` (`GameplayStatics.GetPlayerCameraManager` 0)))
  (`GameplayStatics.SpawnEmitterAttached` (`self.MuzzleEffect`) (`self.Mesh`) "MuzzleFlashSocket")
  (cast `Pawn` (`self.GetOwner`))
  (bind (_outhit _returnvalue_2) (`KismetSystemLibrary.LineTraceSingle` _returnvalue (+ _returnvalue (* (`KismetMathLibrary.GetForwardVector` (`.OutRotation` (`self.GetActorEyesViewPoint` (`GameplayStatics.GetPlayerController` 0)))) (`self.MaxRange`))) "TraceTypeQuery3"))
  (if _returnvalue_2
    (`GameplayStatics.SpawnEmitterAtLocation` (`self.MuzzleSplash`) (`.Location` (`GameplayStatics.BreakHitResult` _outhit)))))

(fn `UserConstructionScript`)