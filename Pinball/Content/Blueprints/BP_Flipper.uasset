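; Flipper Blueprint that sets up a left- or right-sided flipper at construction time from its Type.
; The construction script mirrors the root on X for Right and resets its scale for Left.
; Only the Right branch also sets start and end rotations and applies the start rotation to the mesh.
; BeginPlay is empty, and a timed loop alternating Flip and Flop calls is left disconnected.
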(event `self.ReceiveBeginPlay`)

(fn `UserConstructionScript`
  (bind _rootcomp (`self.RootComp`))
  (switch `EFlipperType` (`self.Type`)
    (:`Right`
      (`SceneComponent.SetRelativeScale3D` _rootcomp (-1.0 1.0 1.0))
      (set `self.StartRotation` (select `EFlipperType` (`self.Type`) :`Right` (struct :`Yaw` 20.0) :`Left` (struct :`Yaw` -20.0) :!type "Rotator Structure"))
      (set `self.EndRotation` (select `EFlipperType` (`self.Type`) :`Right` (struct :`Yaw` -20.0) :`Left` (struct :`Yaw` 20.0) :!type "Rotator Structure"))
      (`SceneComponent.K2_SetRelativeRotation` (`self.MeshComp`) (`self.StartRotation`) false false))
    (:`Left`
      (`SceneComponent.SetRelativeScale3D` _rootcomp (1.0 1.0 1.0)))))