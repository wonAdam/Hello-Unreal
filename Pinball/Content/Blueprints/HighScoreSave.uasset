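; High score data asset that holds an array of score entries and provides functions to rank them.
; Linear scans find the lowest and highest scores, returning an entry and its index.
; Both scans fetch the returned entry using the score value as array index, rather than the found index.
; SortSaveData repeatedly moves the highest result into a temporary array, intending descending order, then copies it back.
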(fn `DetermineHighestScore`
  (returns (HighesttScoreStruct :type "/Game/Blueprints/HighScoreStruct Structure") (HighestScoreIndex :type Integer))
  (locals (HighestScore :type Integer) (HighestIndex :type Integer :default 0))
  (for (_array_element _array_index) (`self.SaveStruct`)
    (if (> (`.Score_5_05247ECB4D714A82AB52B18658DE15DC` (break `/Game/Blueprints/HighScoreStruct` _array_element)) (`local.HighestScore`))
      (set `local.HighestScore` (`.Score_5_05247ECB4D714A82AB52B18658DE15DC` (break `/Game/Blueprints/HighScoreStruct` _array_element)))
      (set `local.HighestIndex` _array_index)))
  (return (`|GetArrayItem` (`self.SaveStruct`) (`local.HighestScore`)) (`local.HighestIndex`)))

(fn `DetermineLowestScore`
  (returns (LowestScoreStruct :type "/Game/Blueprints/HighScoreStruct Structure") (LowestScoreIndex :type Integer))
  (locals (LowestScore :type Integer) (LowestIndex :type Integer :default 0))
  (for (_array_element _array_index) (`self.SaveStruct`)
    (if (< (`.Score_5_05247ECB4D714A82AB52B18658DE15DC` (break `/Game/Blueprints/HighScoreStruct` _array_element)) (`local.LowestScore`))
      (set `local.LowestScore` (`.Score_5_05247ECB4D714A82AB52B18658DE15DC` (break `/Game/Blueprints/HighScoreStruct` _array_element)))
      (set `local.LowestIndex` _array_index)))
  (return (`|GetArrayItem` (`self.SaveStruct`) (`local.LowestScore`)) (`local.LowestIndex`)))

(fn `SortSaveData`
  (locals (TempSaveStruct :type "Array of /Game/Blueprints/HighScoreStruct Structure"))
  (while (> (`KismetArrayLibrary.Array_Length` (`self.SaveStruct`)) 0)
    (bind (_highesttscorestruct _highestscoreindex) (`self.DetermineHighestScore`))
    (`KismetArrayLibrary.Array_Add` (`local.TempSaveStruct`) _highesttscorestruct)
    (`KismetArrayLibrary.Array_Remove` (`self.SaveStruct`) _highestscoreindex))
  (set `self.SaveStruct` (`local.TempSaveStruct`)))