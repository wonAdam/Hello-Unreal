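; BP_Plunger is a plunger actor that pulls back and releases, likely to launch a spawned ball.
; ChargePlunger plays a timeline that lerps the mesh's relative location along local Y from rest to a pulled-back offset.
; StopCharge halts the timeline and uses MoveComponentTo to quickly return the mesh.
; GetBallSpawningLocation converts BallLocation from the actor's local space to world space for ball spawning.
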(event `self.ChargePlunger`
  (bind (_direction _chargealpha) (`Timeline|Charge TImeline` :!via `PlayFromStart` :!label _label)
    (:`Update`
      (`SceneComponent.K2_SetRelativeLocation` (`self.MeshComp`) (`KismetMathLibrary.VLerp` (0.0 0.0 0.0) (0.0 150.0 0.0) _chargealpha) false false))))

(event `self.StopCharge`
  (`|ExecutionSequence`
    (:`then_0`
      (goto _label :!via `Stop`))
    (:`then_1`
      (`KismetSystemLibrary.MoveComponentTo` (`self.MeshComp`) (0.0 0.0 0.0) (struct) false false 0.1))))

(fn `GetBallSpawningLocation`
  (returns (ReturnValue :type "Vector Structure"))
  (return (`KismetMathLibrary.TransformLocation` (`self.GetTransform`) (`self.BallLocation`))))

(fn `UserConstructionScript`)